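; BP_PlayerCube is a player cube that tips over its bottom edge in a given direction to roll across the ground.
; RollUp ignores calls while rolling, otherwise stores the start transform and derives the edge pivot and perpendicular axis, then starts a looping timer.
; MoveTween rotates location and orientation around that pivot in five timed steps toward 90 degrees, though the last applied step is 72, then clears the timer and rolling flag.
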(fn `MoveTween`
  (bind _output_get (set `self.stepPerc` (/ (`KismetMathLibrary.Conv_IntToDouble` (`self.StepCount`)) (`KismetMathLibrary.Conv_IntToDouble` (`self.StepMax`)))))
  (bind _returnvalue (* _output_get 90.0))
  (`self.K2_SetActorLocationAndRotation` (+ (`KismetMathLibrary.RotateAngleAxis` (- (`self.StartLocation`) (`self.PivotPoint`)) _returnvalue (`self.RotationAxis`)) (`self.PivotPoint`)) (`KismetMathLibrary.ComposeRotators` (`self.StartRocation`) (`KismetMathLibrary.RotatorFromAxisAndAngle` (`self.RotationAxis`) _returnvalue)))
  (set `self.StepCount` (+ (`self.StepCount`) 1))
  (if (>= (`self.StepCount`) (`self.StepMax`))
    (`KismetSystemLibrary.K2_ClearTimer` null "MoveTween")
    (set `self.isRolling` false)))

(fn `RollUp`
  (params (Direction :type "Vector Structure"))
  (bind (_direc_x _direc_y) (`KismetMathLibrary.BreakVector` (`self.Direc`)))
  (if (`self.isRolling`)
    (return)
    (else
      (set `self.isRolling` true)
      (set `self.Direc` Direction)
      (set `self.StepMax` 5)
      (set `self.StepCount` 0)
      (set `self.StartLocation` (`self.K2_GetActorLocation`))
      (set `self.StartRocation` (`self.K2_GetActorRotation`))
      (set `self.PivotPoint` (+ (+ (`self.StartLocation`) (* (`self.Direc`) 50.0)) (0.0 0.0 -50.0)))
      (set `self.RotationAxis` (`KismetMathLibrary.MakeVector` _direc_y (* _direc_x -1.0)))
      (`KismetSystemLibrary.K2_SetTimer` null "MoveTween" 0.02 true))))

(fn `UserConstructionScript`)