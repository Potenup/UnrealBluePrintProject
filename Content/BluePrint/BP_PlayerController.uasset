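; Player controller that turns directional input into rolling moves for the player's cube pawn, BP_PlayerCube.
; On BeginPlay it adds the IMC_Input Enhanced Input mapping context, provided the player pawn is that cube.
; Up, down, left and right actions each cast the controlled pawn and call its RollUp with a unit X or Y direction.
; The up action also prints a "Hello" debug string.
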(event `self.ReceiveBeginPlay`
  (cast `/Game/BluePrint/BP_PlayerCube` (`GameplayStatics.GetPlayerPawn` 0))
  (`EnhancedInputSubsystemInterface.AddMappingContext` (subsystem `EnhancedInputLocalPlayerSubsystem`) "/Game/ThirdPerson/Input/IMC_Input.IMC_Input" 0 (struct)))

(event `EnhancedInput|/Game/ThirdPerson/Input/Actions/DPad/IA_UP`
  (params (ActionValue :type Boolean) (ElapsedSeconds :type "Float (double-precision)") (TriggeredSeconds :type "Float (double-precision)") (InputAction :type "InputAction Object Reference" :default "/Game/ThirdPerson/Input/Actions/DPad/IA_UP.IA_UP"))
  (:`Triggered`
    (`KismetSystemLibrary.PrintString` "Hello")
    (bind _asbp_player_cube (cast `/Game/BluePrint/BP_PlayerCube` (`self.K2_GetPawn`)))
    (`/Game/BluePrint/BP_PlayerCube.RollUp` _asbp_player_cube (1.0 0.0 0.0))))

(event `EnhancedInput|/Game/ThirdPerson/Input/Actions/DPad/IA_DOWN`
  (params (ActionValue :type Boolean) (ElapsedSeconds :type "Float (double-precision)") (TriggeredSeconds :type "Float (double-precision)") (InputAction :type "InputAction Object Reference" :default "/Game/ThirdPerson/Input/Actions/DPad/IA_DOWN.IA_DOWN"))
  (:`Triggered`
    (bind _asbp_player_cube (cast `/Game/BluePrint/BP_PlayerCube` (`self.K2_GetPawn`)))
    (`/Game/BluePrint/BP_PlayerCube.RollUp` _asbp_player_cube (-1.0 0.0 0.0))))

(event `EnhancedInput|/Game/ThirdPerson/Input/Actions/DPad/IA_LEFT`
  (params (ActionValue :type Boolean) (ElapsedSeconds :type "Float (double-precision)") (TriggeredSeconds :type "Float (double-precision)") (InputAction :type "InputAction Object Reference" :default "/Game/ThirdPerson/Input/Actions/DPad/IA_LEFT.IA_LEFT"))
  (:`Triggered`
    (bind _asbp_player_cube (cast `/Game/BluePrint/BP_PlayerCube` (`self.K2_GetPawn`)))
    (`/Game/BluePrint/BP_PlayerCube.RollUp` _asbp_player_cube (0.0 -1.0 0.0))))

(event `EnhancedInput|/Game/ThirdPerson/Input/Actions/DPad/IA_RIGHT`
  (params (ActionValue :type Boolean) (ElapsedSeconds :type "Float (double-precision)") (TriggeredSeconds :type "Float (double-precision)") (InputAction :type "InputAction Object Reference" :default "/Game/ThirdPerson/Input/Actions/DPad/IA_RIGHT.IA_RIGHT"))
  (:`Triggered`
    (bind _asbp_player_cube (cast `/Game/BluePrint/BP_PlayerCube` (`self.K2_GetPawn`)))
    (`/Game/BluePrint/BP_PlayerCube.RollUp` _asbp_player_cube (0.0 1.0 0.0))))

(fn `UserConstructionScript`)